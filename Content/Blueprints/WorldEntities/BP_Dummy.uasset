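; Target dummy world entity that displays incoming damage and healing as numbers without tracking any health.
; BeginPlay creates a damage number widget and assigns it to the DamageNumber component, and Damage and Heal forward their amounts to it.
; Inflict passes status effects to the status effect manager component, while a takedamage event applies a fixed hit through Damage.
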(event Custom|takedamage
  (CallFunction|Damage (Utilities|Struct|MakeF_Damage 159.0 0 "0.000000,0.000000,0.000000" false 0)))

(event EventBeginPlay
  (bind _returnvalue (UserInterface|CreateWidget "/Game/Blueprints/Widgets/WBP_DamageNumber.WBP_DamageNumber_C"))
  (UserInterface|SetWidget (Variables|Default|GetDamageNumber) _returnvalue)
  (Variables|Default|SetDamageNumberWidget _returnvalue))

(event EventHeal
  (params (Amount :type Float%20%28double-precision%29))
  (Default|OnHeal (Variables|Default|GetDamageNumberWidget) Amount))

(event EventTick
  (params (DeltaSeconds :type Float%20%28single-precision%29)))

(fn ConstructionScript)

(fn Damage
  (params (Damage%20Info :type F%20Damage%20Structure))
  (Default|OnHit (Variables|Default|GetDamageNumberWidget) (.amount Damage%20Info))
  (return true))

(fn Inflict
  (params (Status%20Effect :type F%20Status%20Effect%20Structure))
  (Default|AddEffect (Variables|Default|GetBPC_StatusEffectManager) Status%20Effect)
  (return))