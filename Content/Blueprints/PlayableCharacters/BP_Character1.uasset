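; BP_Character1 is a playable character Blueprint with an early-stage attack system.
; The standard attack runs a debug-drawn multi box trace along the mesh's forward vector, using the mesh's world location as box half-size.
; Hit actors accumulate uniquely in HitActors, which is never cleared here, and each receives a DamageMessage.
; Special and ultimate attacks only print placeholder text, and the slash montage call is unconnected.
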(event EventTick
  (params (DeltaSeconds :type Float%20%28single-precision%29)))

(event EventDoStandardAttack
  (bind _mesh (Variables|Character|GetMesh))
  (bind _returnvalue (Transformation|GetWorldLocation _mesh))
  ;[0.15 0.15 0.15 0.5] Standard attack system
  (Development|PrintString "standard")
  (bind _outhits (Class|KismetSystemLibrary|BoxTraceMulti _returnvalue (+ _returnvalue (* (Math|Vector|GetForwardVector (Transformation|GetWorldRotation _mesh)) 1e+01)) _returnvalue "0, 0, 0" "TraceTypeQuery1" false 0 "ForDuration" true))
  (for _array_element _outhits
    (Utilities|Array|AddUnique (Variables|Default|GetHit%20Actors) (.HitActor (Collision|BreakHitResult _array_element))))
  (for _array_element_2 (Variables|Default|GetHit%20Actors)
    (Class|BIDamageable|Damage(Message) _array_element_2 (Utilities|Struct|MakeF_Damage 1.0 0 "0.000000,0.000000,0.000000" false 0))))

(event EventDoSpecialAttack
  (Development|PrintString "special"))

(event EventDoUltimateAttack
  (Development|PrintString "ultimate"))

(fn ConstructionScript
  (|CallParentFunction))