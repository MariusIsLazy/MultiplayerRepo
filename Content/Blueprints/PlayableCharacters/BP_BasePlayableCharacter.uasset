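; Base playable character with stick-driven move and aim, a dash along last input, and placeholder standard, special and ultimate attacks meant for overriding.
; The construction script loads health, mana, speed and dash stats from the selected character.
; Damage affecting players updates health, triggers death at zero, passes status effects to a manager component and applies knockback.
; A separate Damaged event animates global time dilation, and the example special spawns an AOE cloud under the cursor.
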(event EventSecondaryThumbstick
  (params (Axis :type Vector%202D%20Structure))
  ;[0.15 0.15 0.15 0.5] Touch Inputs
  (Class|TwinStickCharacter|DoAim (.y Axis) (.x Axis)))

(event EventHeal
  (params (Amount :type Float%20%28double-precision%29))
  (CallFunction|UpdateHealth (Math|Float|Min(Float) (+ Amount (Variables|State|GetHealth)) (Variables|BaseStats|GetMaxHealth))))

(event EventDoStandardAttack
  (Development|PrintString "Standard, Override me!"))

(event EventDoSpecialAttack
  (Development|PrintString "Special, Override me!")
  (CallFunction|ExampleSpecialAttack))

(event EventDoUltimateAttack
  (Development|PrintString "Ultimate, override me!"))

(event EventDamaged
  ;[0.15 0.15 0.15 0.5] Apply time dilation when the player character is damaged
  (bind _time_dilation (Timeline|Damaged%20Timeline PlayFromStart)
    (:Update
      (Utilities|Time|SetGlobalTimeDilation _time_dilation))
    (:Finished
      (Utilities|Time|SetGlobalTimeDilation 1.0))))

(event EventPrimaryThumbstick
  (params (Axis :type Vector%202D%20Structure))
  ;[0.15 0.15 0.15 0.5] Touch Inputs
  (Class|TwinStickCharacter|DoMove (.y Axis) (.x Axis)))

(event EventDoDash
  (bind _charactermovement (Variables|Character|GetCharacterMovement))
  (bind _bonusdashdistance (Variables|UpgradeStats|GetBonusDashDistance))
  (bind _dashdistance (Variables|BaseStats|GetDashDistance))
  (bind _returnvalue (Pawn|Components|PawnMovement|GetLastInputVector _charactermovement))
  (bind _returnvalue_2 (+ _bonusdashdistance _dashdistance))
  (Character|LaunchCharacter (Math|Vector|MakeVector (* (.x _returnvalue) _returnvalue_2) (* (.y _returnvalue) _returnvalue_2) 0.0) false false))

(fn ConstructionScript
  (CallFunction|SetBaseStats (CallFunction|GetSelectedCharacterStats)))

(fn UpdateHealth
  (params (NewHealth :type Float%20%28double-precision%29))
  (bind _output_get (Variables|State|SetHealth NewHealth))
  ;[0.15 0.15 0.15 0.5] Logic to check if dead
  (if (<= _output_get 0.0)
    (CallFunction|OnDeath)
    (Default|CallDeath)))

(fn SetBaseStats
  (params (Character%20Stats :type ST%20Character%20Stats%20Structure))
  (Utilities|FlowControl|Sequence
    (:then_0
      (Variables|BaseStats|SetMaxHealth (.maxhealth Character%20Stats))
      (Variables|BaseStats|SetMaxMana (.maxmana Character%20Stats))
      (Variables|BaseStats|SetDashDistance (.dashdistance Character%20Stats))
      (Variables|BaseStats|SetMovementSpeed (.movementspeed Character%20Stats))
      (Variables|Default|SetCharacterName (.charactername Character%20Stats)))
    (:then_1
      (Variables|/Script/Engine.CharacterMovementComponent|SetMaxWalkSpeed (Variables|Character|GetCharacterMovement) (Variables|BaseStats|GetMovementSpeed))
      (Variables|State|SetHealth (Variables|BaseStats|GetMaxHealth))
      (Variables|State|SetMana (Variables|BaseStats|GetMaxMana)))))

(fn ExampleSpecialAttack
  (Game|SpawnActorfromClass "/Game/Blueprints/CombatEntities/BP_AOECloud.BP_AOECloud_C" (Math|Transform|MakeTransform (.location (.HitResult (Game|Player|GetHitResultUnderCursorbyChannel (Pawn|GetLocalViewingPlayerController) "TraceTypeQuery1" true))) "0, 0, 0" "1.000000,1.000000,1.000000") "Undefined" "MultiplyWithRoot" 0 self))

(fn OnDeath)

(fn Damage
  (params (Damage%20Info :type F%20Damage%20Structure))
  (if (.affectsplayers Damage%20Info)
    (Utilities|FlowControl|Sequence
      (:then_0
        ;[0.15 0.15 0.15 0.5] Health
        (CallFunction|UpdateHealth (- (Variables|State|GetHealth) (.Amount (Utilities|Struct|BreakF_Damage Damage%20Info)))))
      (:then_1
        ;[0.15 0.15 0.15 0.5] Status Effects
        (for _array_element (.inflictsstatuseffects Damage%20Info)
          (CallFunction|Inflict _array_element)))
      (:then_2
        ;[0.15 0.15 0.15 0.5] Knockback
        (Physics|AddImpulse (Variables|Character|GetCharacterMovement) (.knockback Damage%20Info) false))
      (:then_3
        ;[0.15 0.15 0.15 0.5] UI hurt response
        (if true
          _))
      (:then_4
        ;[0.15 0.15 0.15 0.5] Finish
        (return true)))
    (else
      (return false))))

(fn Inflict
  (params (Status%20Effect :type F%20Status%20Effect%20Structure))
  (Default|AddEffect (Variables|Default|GetBPC_StatusEffectManager) Status%20Effect)
  (return))