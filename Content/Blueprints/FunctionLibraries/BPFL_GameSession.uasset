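; Blueprint function library for session-wide access to the player's selected character.
; Each function casts the current Game Instance to BP_GameInstance and forwards the call to it.
; It sets the selection from a character data row name and returns the selected character's stats and class.
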(fn SetSelectedCharacter
  (params (SelectedCharacterDataRow :type Name))
  (bind _asbp_game_instance (Utilities|Casting|CastToBP_GameInstance (Game|GetGameInstance (LocalVariables|Get__WorldContext))))
  (Default|SetSelectedCharacterClassbyName _asbp_game_instance SelectedCharacterDataRow))

(fn GetSelectedCharacterStats
  (bind _asbp_game_instance (Utilities|Casting|CastToBP_GameInstance (Game|GetGameInstance (LocalVariables|Get__WorldContext))))
  (bind _selectedcharacterbasestats (Default|GetSelectedCharacterStats _asbp_game_instance))
  (return _selectedcharacterbasestats))

(fn GetSelectedCharacterClass
  (bind _asbp_game_instance (Utilities|Casting|CastToBP_GameInstance (Game|GetGameInstance (LocalVariables|Get__WorldContext))))
  (bind _selected_character_base_stats_character_class (Default|GetSelectedCharacterClass _asbp_game_instance))
  (return _selected_character_base_stats_character_class))