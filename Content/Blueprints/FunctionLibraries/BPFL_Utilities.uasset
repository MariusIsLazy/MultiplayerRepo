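; Blueprint function library with helpers that build damage data and status effect objects.
; MakeDamage packs amount, status effects, player-affect flag and source, deriving knockback from the normalized source-to-target direction scaled by the knockback amount.
; MakeStatusEffect constructs an object whose class is selected by effect type, then copies type, duration, strength and the initial struct onto it.
; Only Regeneration maps to its own subclass; other types use the base BP_StatusEffect.
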(fn MakeDamage
  (params (Damage%20Amount :type Float%20%28double-precision%29) (KnockbackAmount :type Float%20%28double-precision%29) (%20Inflicts%20Status%20Effects :type Array%20of%20F%20Status%20Effect%20Structures) (%20Affects%20Players :type Boolean) (%20Source :type Actor%20Object%20Reference) (Target :type Actor%20Object%20Reference))
  (return (Utilities|Struct|MakeF_Damage Damage%20Amount %20Inflicts%20Status%20Effects (* (Math|Vector|Normalize (- (Transformation|GetActorLocation Target) (Transformation|GetActorLocation %20Source))) KnockbackAmount) %20Affects%20Players %20Source)))

(fn MakeStatusEffect
  (params (FStatusEffect :type F%20Status%20Effect%20Structure))
  (bind _returnvalue (Game|ConstructObjectfromClass (LocalVariables|Get__WorldContext) (Utilities|Select :Index (.effect FStatusEffect) :NewEnumerator0 "/Game/Blueprints/Effects/BP_StatusEffect.BP_StatusEffect_C" :NewEnumerator1 "/Game/Blueprints/Effects/BP_StatusEffect.BP_StatusEffect_C" :NewEnumerator2 "/Game/Blueprints/Effects/BP_StatusEffect.BP_StatusEffect_C" :NewEnumerator3 "/Game/Blueprints/Effects/BP_StatusEffect.BP_StatusEffect_C" :NewEnumerator4 "/Game/Blueprints/Effects/BP_StatusEffect_Regeneration.BP_StatusEffect_Regeneration_C" :NewEnumerator5 "/Game/Blueprints/Effects/BP_StatusEffect.BP_StatusEffect_C")))
  (bind _asbp_status_effect (Utilities|Casting|CastToBP_StatusEffect _returnvalue))
  (Variables|/Game/Blueprints/Effects/BP_StatusEffect.BP_StatusEffect_C|SetStatus%20Effect%20Type _asbp_status_effect (.effect FStatusEffect))
  (Variables|/Game/Blueprints/Effects/BP_StatusEffect.BP_StatusEffect_C|SetDuration _asbp_status_effect (.duration FStatusEffect))
  (Variables|/Game/Blueprints/Effects/BP_StatusEffect.BP_StatusEffect_C|SetStrength _asbp_status_effect (.strength FStatusEffect))
  (Variables|/Game/Blueprints/Effects/BP_StatusEffect.BP_StatusEffect_C|SetInitialEffectStats _asbp_status_effect FStatusEffect)
  (return _asbp_status_effect))