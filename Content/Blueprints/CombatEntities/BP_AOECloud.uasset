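; BP_AOECloud is a timed area-of-effect cloud that applies a status effect to damageable actors inside it.
; Cylinder overlap events maintain a list of actors implementing BI_Damageable, adding them on entry and removing them on exit.
; A looping timer, set by the tick rate, inflicts a fixed status effect on each listed actor until the cloud's lifespan expires.
; Older direct-damage logic remains but is disconnected.
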(event OnComponentBeginOverlap(Cylinder)
  (params (OverlappedComponent :type Primitive%20Component%20Object%20Reference) (OtherActor :type Actor%20Object%20Reference) (OtherComp :type Primitive%20Component%20Object%20Reference) (OtherBodyIndex :type Integer) (bFromSweep :type Boolean) (SweepResult :type Hit%20Result%20Structure%20%28by%20ref%29))
  ;[0.15 0.15 0.15 0.5] Get overlapping actors
  (bind _asbi_damageable (Utilities|Casting|CastToBI_Damageable OtherActor))
  (Utilities|Array|AddUnique (Variables|Default|GetOverlapping%20Damagables) _asbi_damageable))

(event OnComponentEndOverlap(Cylinder)
  (params (OverlappedComponent :type Primitive%20Component%20Object%20Reference) (OtherActor :type Actor%20Object%20Reference) (OtherComp :type Primitive%20Component%20Object%20Reference) (OtherBodyIndex :type Integer))
  ;[0.15 0.15 0.15 0.5] Get overlapping actors
  (bind _asbi_damageable (Utilities|Casting|CastToBI_Damageable OtherActor))
  (Utilities|Array|RemoveItem (Variables|Default|GetOverlapping%20Damagables) _asbi_damageable))

(event Custom|OnTick
  ;[0.15 0.15 0.15 0.5] Damage all damagables overlapping
  (for _array_element (Variables|Default|GetOverlapping%20Damagables)
    (Default|Inflict _array_element (Utilities|Struct|MakeF_StatusEffect "NewEnumerator4" 5.0 1.0))))

(event EventBeginPlay
  (Utilities|Time|SetTimerbyEvent (delegate Custom|OnTick) (/ 1.0 (Variables|Default|GetTickRatePerSecond)) true true)
  (Actor|SetLifeSpan (Variables|Default|GetLifetime)))

(fn ConstructionScript)