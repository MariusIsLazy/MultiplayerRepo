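; Regeneration status effect that periodically heals its Owner.
; Tick counts a timer down by delta time, then resets it to Interval and calls Heal whenever it runs out.
; Heal sends a HealMessage carrying Strength to the Owner and prints a debug string, using the Owner as world context.
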(fn Tick
  (params (Delta%20Seconds :type Float%20%28double-precision%29))
  (bind _output_get (Variables|Default|SetTimeToNextHeal (- (Variables|Default|GetTimeToNextHeal) Delta%20Seconds)))
  (if (<= _output_get 0.0)
    (Variables|Default|SetTimeToNextHeal (Variables|Default|GetInterval))
    (CallFunction|Heal)))

(fn Heal
  (bind _owner (Variables|Default|GetOwner))
  (Class|BIDamageable|Heal(Message) _owner (Variables|Default|GetStrength))
  (Development|PrintString _owner "Healing"))