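; Base status effect Blueprint that gives a timed effect on an owner a common lifecycle.
; Start stores the Owner, while Tick and End are empty stubs for the effect's own behavior.
; LifeTick counts Duration down by delta time, and once it drops below zero calls End and fires the LifeEnd dispatcher with itself.
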(fn Start
  (params (Owner :type Actor%20Object%20Reference))
  (Variables|Default|SetOwner Owner))

(fn Tick
  (params (Delta%20Seconds :type Float%20%28double-precision%29)))

(fn End)

(fn LifeTick
  (params (Delta%20Seconds :type Float%20%28double-precision%29))
  (bind _output_get (Variables|Default|SetDuration (- (Variables|Default|GetDuration) Delta%20Seconds)))
  (if (< _output_get 0.0)
    (CallFunction|End)
    (Default|CallLifeEnd self)))