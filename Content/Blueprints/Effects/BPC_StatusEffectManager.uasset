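; Actor component that manages the timed status effects active on its owner.
; AddEffect looks up an effect of the same type: equal strength keeps the longer duration, greater strength replaces it, and weaker is ignored.
; New effect objects start on the owner, join CurrentEffects and get an event bound to their life end.
; The component's Tick drives each effect's behavior and lifetime ticks.
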(event EventBeginPlay)

(event EventTick
  (params (DeltaSeconds :type Float%20%28single-precision%29))
  (for _array_element (Variables|Default|GetCurrentEffects)
    (Default|Tick _array_element DeltaSeconds)
    (Default|LifeTick _array_element DeltaSeconds)))

(fn AddEffect
  (params (Status%20Effect :type F%20Status%20Effect%20Structure))
  (bind (_effect _found) (CallFunction|FindEffect (.effect Status%20Effect)))
  (LocalVariables|SetFoundEffect _effect)
  (if _found
    (if (>= (.strength Status%20Effect) (Variables|/Game/Blueprints/Effects/BP_StatusEffect.BP_StatusEffect_C|GetStrength (LocalVariables|GetFoundEffect)))
      (if (== (.strength Status%20Effect) (Variables|/Game/Blueprints/Effects/BP_StatusEffect.BP_StatusEffect_C|GetStrength (LocalVariables|GetFoundEffect)))
        ;[0.15 1 0 0.5] Update Effect if strength is equal
        (Variables|/Game/Blueprints/Effects/BP_StatusEffect.BP_StatusEffect_C|SetDuration (LocalVariables|GetFoundEffect) (Math|Float|Max(Float) (.duration Status%20Effect) (Variables|/Game/Blueprints/Effects/BP_StatusEffect.BP_StatusEffect_C|GetDuration (LocalVariables|GetFoundEffect))))
        (Development|PrintString "Updated effect")
        (elif (> (.strength Status%20Effect) (Variables|/Game/Blueprints/Effects/BP_StatusEffect.BP_StatusEffect_C|GetStrength (LocalVariables|GetFoundEffect)))
          ;[0.3092 0 0.7739 0.5] Upgrade Effect if strength is greater
          (CallFunction|RemoveEffect (LocalVariables|GetFoundEffect))
          (bind _effect_object (CallFunction|MakeStatusEffect Status%20Effect))
          (CallFunction|StartEffect _effect_object)
          (Development|PrintString "Upgraded effect"))))
    (else
      (bind _effect_object_2 (CallFunction|MakeStatusEffect Status%20Effect))
      (CallFunction|StartEffect _effect_object_2)
      (Development|PrintString "Created effect"))))

(fn FindEffect
  (params (Effect%20Type :type E_StatusEffect%20Enum :default "NewEnumerator0"))
  (Utilities|FlowControl|Sequence
    (:then_0
      (bind _array_element (Utilities|Array|ForEachLoopwithBreak (Variables|Default|GetCurrentEffects) :!label _label)
        (:LoopBody
          (if (Utilities|Enum|Equal(Enum) (Variables|/Game/Blueprints/Effects/BP_StatusEffect.BP_StatusEffect_C|GetStatus%20Effect%20Type _array_element) Effect%20Type)
            (LocalVariables|SetEffectObject _array_element)
            (LocalVariables|SetwasEffectFound (Utilities|Enum|Equal(Enum) (Variables|/Game/Blueprints/Effects/BP_StatusEffect.BP_StatusEffect_C|GetStatus%20Effect%20Type _array_element) Effect%20Type))
            (goto _label Break)))))
    (:then_1
      (return (LocalVariables|GetEffectObject) (LocalVariables|GetwasEffectFound)))))

(fn StartEffect
  (params (EffectObject :type BP%20Status%20Effect%20Object%20Reference))
  (Default|Start EffectObject (Components|GetOwner))
  (Utilities|Array|AddUnique (Variables|Default|GetCurrentEffects) EffectObject)
  (EventDispatchers|BindEventtoLifeEnd EffectObject (EventDispatchers|CreateEvent :!event RemoveEffect)))

(fn RemoveEffect
  (params (EffectObject :type BP%20Status%20Effect%20Object%20Reference))
  (Utilities|Array|RemoveItem (Variables|Default|GetCurrentEffects) EffectObject))