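; Escort objective actor that moves an escort item along a spline while a player-controlled pawn is within range.
; Once started, server-side Tick scans all pawns for a player inside the escort radius and advances progress by delta time over travel duration.
; At the spline's end it marks the escort complete and notifies the enemy spawner to complete the objective.
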(event Custom|StartEscort
  ;[0.15 0.15 0.15 0.5] Starting the escort
  (Networking|SwitchHasAuthority
    (:Authority
      (if (not (Variables|Default|GetEscortStarted))
        (Variables|Default|SetEscortStarted true)))))

(event Custom|MCMoveBox
  (bind _escortpath (Variables|Default|GetEscortPath))
  (Variables|Default|SetTravelProgress (Math|Float|Clamp(Float) (+ (/ (Utilities|Time|GetWorldDeltaSeconds) (Variables|Default|GetTravelDuration)) (Variables|Default|GetTravelProgress))))
  (Transformation|SetWorldLocation (Variables|Default|GetEscortItem) (Spline|GetLocationatDistanceAlongSpline _escortpath (* (Spline|GetSplineLength _escortpath) (Variables|Default|GetTravelProgress)) "World") false false)
  (if (>= (Variables|Default|GetTravelProgress) 1.0)
    (Variables|Default|SetEscortComplete true)
    (Default|CompleteObjective (Variables|Default|GetEnemySpawner))
    (Development|PrintString "escort complete")))

(event EventBeginPlay
  ;[0.15 0.15 0.15 0.5] Begin Play
  (Transformation|SetWorldLocation (Variables|Default|GetEscortItem) (Spline|GetLocationatDistanceAlongSpline (Variables|Default|GetEscortPath) 0.0 "World") false false))

(event EventTick
  (params (DeltaSeconds :type Float%20%28single-precision%29))
  ;[0.15 0.15 0.15 0.5] Update event tick for the object moving
  (Networking|SwitchHasAuthority
    (:Authority
      (if (Variables|Default|GetEscortStarted)
        (if (not (Variables|Default|GetEscortComplete))
          (bind _playernearby (CallFunction|IsPlayerNearEscort))
          (if _playernearby
            (CallFunction|MCMoveBox)))))))

(fn ConstructionScript)

(fn IsPlayerNearEscort
  ;[0.15 0.15 0.15 0.5] Radius check to move the objective
  (Variables|Default|SetFoundPlayer false)
  (bind _outactors (Actor|GetAllActorsOfClass "/Script/Engine.Pawn"))
  (for _array_element _outactors
    (if (Pawn|IsPlayerControlled _array_element)
      (if (<= (Math|Vector|Distance(Vector) (Transformation|GetActorLocation _array_element) (Transformation|GetWorldLocation (Variables|Default|GetEscortItem))) (Variables|Default|GetEscortRadius))
        (Variables|Default|SetFoundPlayer true))))
  (return (Variables|Default|GetFoundPlayer)))