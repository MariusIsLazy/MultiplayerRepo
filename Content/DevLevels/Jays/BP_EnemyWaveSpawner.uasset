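; BP_EnemyWaveSpawner is a trigger volume actor that runs repeating enemy waves during an escort objective.
; When a player-controlled pawn overlaps its box, the server starts once: it spawns a wave, starts a looping timer and starts the linked escort.
; Each wave spawns a BP_EnemyBase at ten spawn-point components, nudged to avoid collisions or skipped.
; CompleteObjective flags completion and clears the timer to end spawning.
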(event OnComponentBeginOverlap(Box)
  (params (OverlappedComponent :type Primitive%20Component%20Object%20Reference) (OtherActor :type Actor%20Object%20Reference) (OtherComp :type Primitive%20Component%20Object%20Reference) (OtherBodyIndex :type Integer) (bFromSweep :type Boolean) (SweepResult :type Hit%20Result%20Structure%20%28by%20ref%29))
  ;[0.15 0.15 0.15 0.5] Overlap to start the spawner
  (Networking|SwitchHasAuthority
    (:Authority
      (bind _aspawn (Utilities|Casting|CastToPawn OtherActor))
      (if (Pawn|IsPlayerControlled _aspawn)
        (if (not (Variables|Default|GetObjectiveStarted))
          (Variables|Default|SetObjectiveStarted true)
          (CallFunction|SpawnWave)
          (bind _returnvalue (Utilities|Time|SetTimerbyFunctionName 0 "SpawnWave" (Variables|Default|GetWaveInterval) true))
          (Variables|Default|SetWaveTimerHandle _returnvalue)
          (Default|StartEscort (Variables|Default|GetEscortObjective)))))))

(event Custom|SpawnWave
  ;[0.15 0.15 0.15 0.5] Spawner and spawn point
  (if (not (Variables|Default|GetObjectiveComplete))
    (for _array_element (Utilities|Array|MakeArray (Variables|Default|GetSpawnPoint_01) (Variables|Default|GetSpawnPoint_02) (Variables|Default|GetSpawnPoint_03) (Variables|Default|GetSpawnPoint_04) (Variables|Default|GetSpawnPoint_05) (Variables|Default|GetSpawnPoint_06) (Variables|Default|GetSpawnPoint_07) (Variables|Default|GetSpawnPoint_08) (Variables|Default|GetSpawnPoint_09) (Variables|Default|GetSpawnPoint_010))
      (Game|SpawnActorfromClass "/Game/DevLevels/Jays/Enemies/BP_EnemyBase.BP_EnemyBase_C" (Transformation|GetWorldTransform _array_element) "AdjustIfPossibleButDontSpawnIfColliding" "MultiplyWithRoot" 0 0))))

(event Custom|CompleteObjective
  ;[0.15 0.15 0.15 0.5] Objective Complete
  (Variables|Default|SetObjectiveComplete true)
  (Utilities|Time|ClearandInvalidateTimerbyHandle (Variables|Default|GetWaveTimerHandle)))

(fn ConstructionScript)