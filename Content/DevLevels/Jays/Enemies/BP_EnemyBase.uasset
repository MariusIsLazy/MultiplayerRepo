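; Base enemy character with health, melee attacks, hit reactions and death, with gameplay logic gated on server authority.
; The Damage function feeds AnyDamage, which triggers a hit react or death with delayed destroy, while MC_ events play the montages.
; An overlap box, toggled by attack-window events, damages each player once per swing and closes on hit react or death.
; EnemyState behaviour is stubbed, and debug timers can force damage or reactions.
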(event OnComponentBeginOverlap(EnemyAttackBox)
  (params (OverlappedComponent :type Primitive%20Component%20Object%20Reference) (OtherActor :type Actor%20Object%20Reference) (OtherComp :type Primitive%20Component%20Object%20Reference) (OtherBodyIndex :type Integer) (bFromSweep :type Boolean) (SweepResult :type Hit%20Result%20Structure%20%28by%20ref%29))
  (bind _actorshittarget (Variables|Default|GetActorsHitTarget))
  ;[0.15 0.15 0.15 0.5] Hit detection from enemies onto player
  (Networking|SwitchHasAuthority
    (:Authority
      (bind _asbp_base_playable_character (Utilities|Casting|CastToBP_BasePlayableCharacter OtherActor))
      (if (not (Variables|Default|GetIsDead))
        (if (not (Variables|Default|GetIsReacting))
          (if (not (Utilities|Array|ContainsItem _actorshittarget OtherActor))
            (Utilities|Array|AddUnique _actorshittarget OtherActor)
            (Development|PrintString "Enemy Attack Hit Player")
            (Class|BIDamageable|Damage(Message) _asbp_base_playable_character (Utilities|Struct|MakeF_Damage 1e+01 0 "0.000000,0.000000,0.000000" true self))
            (Development|PrintString (Utilities|String|ToString(Float) (Variables|/Game/Blueprints/PlayableCharacters/BP_BasePlayableCharacter.BP_BasePlayableCharacter_C|GetHealth _asbp_base_playable_character)))))))))

(event Custom|MC_PlayAttack
  ;[0.15 0.15 0.15 0.5] Attack
  (Animation|PlayAnimMontage (Variables|Default|GetSwordSwing) 1.0 "None"))

(event Custom|TryAttack
  ;[0.15 0.15 0.15 0.5] Attack Montage
  (Networking|SwitchHasAuthority
    (:Authority
      (if (not (Variables|Default|GetIsDead))
        (if (not (Variables|Default|GetIsAttacking))
          (if (not (Variables|Default|GetIsReacting))
            (Variables|Default|SetIsAttacking true)
            (CallFunction|MCPlayAttack)
            (Utilities|FlowControl|Delay (Math|Float|Max(Float) (Animation|GetPlayLength (Variables|Default|GetAttackMontage)) (Variables|Default|GetAttackCooldown)))
            (Variables|Default|SetIsAttacking false)))))))

(event Custom|MC_PlayHitReact
  ;[0.15 0.15 0.15 0.5] Hit Anim
  (Animation|PlayAnimMontage (Variables|Default|GetHitReactMontage) 1.0 "None"))

(event Custom|TryHitReact
  ;[0.15 0.15 0.15 0.5] Being hit reaction logic
  (Networking|SwitchHasAuthority
    (:Authority
      (if (not (Variables|Default|GetIsDead))
        (if (not (Variables|Default|GetIsReacting))
          (Variables|Default|SetIsReacting true)
          (CallFunction|CloseAttackWindow)
          (bind _asaicontroller (Utilities|Casting|CastToAIController (Pawn|GetController))
            (:then
              (AI|Navigation|StopMovement _asaicontroller))
            (:CastFailed
              _))
          (CallFunction|MCPlayHitReact)
          (Utilities|FlowControl|Delay (Animation|GetPlayLength (Variables|Default|GetHitReactMontage)))
          (Variables|Default|SetIsReacting false))))))

(event Custom|OpenAttackWindow
  ;[0.15 0.15 0.15 0.5] Open Attack Window
  (Networking|SwitchHasAuthority
    (:Authority
      (if (not (Variables|Default|GetIsDead))
        (if (not (Variables|Default|GetIsReacting))
          (if (Variables|Default|GetIsAttacking)
            (Utilities|Array|Clear (Variables|Default|GetActorsHitTarget))
            (Collision|SetCollisionEnabled (Variables|Default|GetEnemyAttackBox) "QueryOnly")))))))

(event Custom|DebugApplyDamage
  ;[0.15 0.15 0.15 0.5] Apply Damage call
  (Game|Damage|ApplyDamage self 1e+01 0 0))

(event Custom|MC_PlayDeath
  ;[0.15 0.15 0.15 0.5] Death Anim / removed capsule
  (Collision|SetCollisionEnabled (Variables|Collision|GetCapsuleComponent) "NoCollision")
  (Animation|PlayAnimMontage (Variables|Default|GetDeathMontage) 1.0 "None"))

(event Custom|CloseAttackWindow
  ;[0.15 0.15 0.15 0.5] Close sttack window
  (Networking|SwitchHasAuthority
    (:Authority
      (Collision|SetCollisionEnabled (Variables|Default|GetEnemyAttackBox) "NoCollision"))))

(event EventBeginPlay
  ;[0.15 0.15 0.15 0.5] BeginPlay and Health
  (Utilities|FlowControl|Sequence
    (:then_0
      (Networking|SwitchHasAuthority
        (:Authority
          (Variables|Default|SetHomeLocation (Transformation|GetActorLocation))
          (Variables|Default|SetHealth (Variables|Default|GetMaxHealth))
          ;[0.15 0.15 0.15 0.5] Used for all debug prints
          (Utilities|FlowControl|Sequence
            (:then_0
              ;[0.15 0.15 0.15 0.5] Debug hit react with logic in "tryhitreact"
              (if (Variables|Default|GetDebugHitReact)
                (Utilities|Time|SetTimerbyFunctionName 0 "TryHitReact" 2.0 true)))
            (:then_1
              ;[0.15 0.15 0.15 0.5] Damage debug
              (if (Variables|Default|GetDebugDamage)
                (Utilities|Time|SetTimerbyFunctionName 0 "DebugApplyDamage" 2.0 true)))))))
    (:then_1
      ;[0.15 0.15 0.15 0.5] Later for enemy states using enums
      (switch Utilities|FlowControl|Switch|SwitchonEnum_EnemyState (Variables|Default|GetEnemyState)))))

(event Game|Damage|EventAnyDamage
  (params (Damage :type Float%20%28single-precision%29) (DamageType :type Damage%20Type%20Object%20Reference) (InstigatedBy :type Controller%20Object%20Reference) (DamageCauser :type Actor%20Object%20Reference))
  ;[0.15 0.15 0.15 0.5] Damage
  (if (not (Variables|Default|GetIsDead))
    (if true
      (bind _output_get (Variables|Default|SetHealth (Math|Float|Clamp(Float) (- (Variables|Default|GetHealth) Damage) 0.0 (Variables|Default|GetMaxHealth))))
      (Development|PrintString (Utilities|String|ToString(Float) _output_get))
      (if (> (Variables|Default|GetHealth) 0.0)
        (CallFunction|TryHitReact)
        (else
          (Variables|Default|SetIsDead true)
          (CallFunction|CloseAttackWindow)
          (Pawn|Components|CharacterMovement|DisableMovement (Variables|Character|GetCharacterMovement))
          (CallFunction|MCPlayDeath)
          (Utilities|FlowControl|Delay 1e+01)
          (Actor|DestroyActor))))))

(fn ConstructionScript
  (switch Utilities|FlowControl|Switch|SwitchonEnum_EnemyState (Variables|Default|GetEnemyState)
    (:NewEnumerator0
      (Components|SkeletalMesh|SetSkeletalMeshAsset (Variables|Character|GetMesh) "/Game/DevLevels/Jays/Enemy_Assets/Survivor_A_Lusth.Survivor_A_Lusth"))
    (:NewEnumerator1
      (Components|SkeletalMesh|SetSkeletalMeshAsset (Variables|Character|GetMesh) "/Game/DevLevels/Jays/Enemy_Assets/Survivor_A_Lusth.Survivor_A_Lusth"))
    (:NewEnumerator2
      (Components|SkeletalMesh|SetSkeletalMeshAsset (Variables|Character|GetMesh) "/Game/DevLevels/Jays/Enemy_Assets/Survivor_A_Lusth.Survivor_A_Lusth"))))

(fn Damage
  (params (Damage%20Info :type F%20Damage%20Structure))
  (Development|PrintString "enemy recieved attack")
  (Networking|SwitchHasAuthority
    (:Authority
      (if (Variables|Default|GetIsDead)
        _
        (elif (> (.amount Damage%20Info) 0.0)
          (Game|Damage|ApplyDamage self (.amount Damage%20Info) 0 0)
          (return true)
          (else
            _))))
    (:Remote
      _))
  (return false))