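; AI controller for BP_EnemyBase enemies that patrols, detects, chases and attacks player-controlled characters.
; On possess, the server targets the nearest player within detection radius, alerts the enemy and starts a looping timer for periodic target checks.
; CheckTarget resumes chasing or stops to attack when in range and facing, while server Tick smooths yaw toward the target.
; Unalerted enemies wander to random reachable points around home.
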(event Custom|ChaseTarget
  ;[0.15 0.15 0.15 0.5] Chase Target
  (Utilities|IsValid (Variables|Default|GetTargetPlayer)
    (:Is%20Valid
      (AI|AIMoveTo (Pawn|GetControlledPawn) "0, 0, 0" (Variables|Default|GetTargetPlayer) 5e+01 false))))

(event Custom|CheckTarget
  (bind _returnvalue (Pawn|GetControlledPawn))
  (bind _targetplayer (Variables|Default|GetTargetPlayer))
  ;[0.15 0.15 0.15 0.5] Target checks
  (Utilities|IsValid (Variables|Default|GetTargetPlayer)
    (:Is%20Valid
      (if (<= (Transformation|GetDistanceTo _returnvalue _targetplayer) (Variables|Default|GetAttackRange))
        (bind _asbp_enemy_base (Utilities|Casting|CastToBP_EnemyBase _returnvalue))
        (AI|Navigation|StopMovement)
        (if (< (Math|Float|Absolute(Float) (.Yaw (Math|Rotator|BreakRotator (Math|Rotator|Delta(Rotator) (Math|Rotator|MakeRotator 0.0 0.0 (.Yaw (Math|Rotator|BreakRotator (Math|Rotator|FindLookatRotation (Transformation|GetActorLocation _returnvalue) (Transformation|GetActorLocation _targetplayer))))) (Transformation|GetActorRotation _returnvalue))))) 15.0)
          (Default|TryAttack _asbp_enemy_base))
        (else
          (bind _asbp_enemy_base_2 (Utilities|Casting|CastToBP_EnemyBase _returnvalue))
          (if (not (Math|Boolean|ORBoolean (Variables|/Game/DevLevels/Jays/Enemies/BP_EnemyBase.BP_EnemyBase_C|GetIsReacting _asbp_enemy_base_2) (Variables|/Game/DevLevels/Jays/Enemies/BP_EnemyBase.BP_EnemyBase_C|GetIsAttacking _asbp_enemy_base_2) (Variables|/Game/DevLevels/Jays/Enemies/BP_EnemyBase.BP_EnemyBase_C|GetIsDead _asbp_enemy_base_2)))
            (if (Utilities|Enum|Equal(Enum) (Class|AIController|GetMoveStatus) "Idle")
              (CallFunction|ChaseTarget))))))
    (:Is%20Not%20Valid
      (CallFunction|FindNearestPlayer)
      (CallFunction|ChaseTarget))))

(event Custom|TryPatrol
  (bind _returnvalue (Pawn|GetControlledPawn))
  ;[0.15 0.15 0.15 0.5] Patrol
  (bind _asbp_enemy_base (Utilities|Casting|CastToBP_EnemyBase _returnvalue))
  (if (not (Variables|/Game/DevLevels/Jays/Enemies/BP_EnemyBase.BP_EnemyBase_C|GetIsDead _asbp_enemy_base))
    (if (not (Variables|/Game/DevLevels/Jays/Enemies/BP_EnemyBase.BP_EnemyBase_C|GetIsAlerted _asbp_enemy_base))
      (if (Utilities|Enum|Equal(Enum) (Variables|/Game/DevLevels/Jays/Enemies/BP_EnemyBase.BP_EnemyBase_C|GetEnemyState _asbp_enemy_base) "NewEnumerator2")
        (if (not (Variables|/Game/DevLevels/Jays/Enemies/BP_EnemyBase.BP_EnemyBase_C|GetIsReacting _asbp_enemy_base))
          (if (not (Variables|/Game/DevLevels/Jays/Enemies/BP_EnemyBase.BP_EnemyBase_C|GetIsAttacking _asbp_enemy_base))
            (bind (_randomlocation _returnvalue_2) (AI|Navigation|GetRandomReachablePointinRadius (Variables|/Game/DevLevels/Jays/Enemies/BP_EnemyBase.BP_EnemyBase_C|GetHomeLocation _asbp_enemy_base) (Variables|/Game/DevLevels/Jays/Enemies/BP_EnemyBase.BP_EnemyBase_C|GetPatrolRadius _asbp_enemy_base) 0 0))
            (if _returnvalue_2
              (Variables|Default|SetPatrolDestination _randomlocation)
              (AI|AIMoveTo _returnvalue (Variables|Default|GetPatrolDestination) 0 5e+01 false
                (:OnSuccess
                  _)
                (:OnFail
                  _)))
            (Utilities|FlowControl|Delay 2.0)
            (CallFunction|TryPatrol)))))))

(event EventTick
  (params (DeltaSeconds :type Float%20%28single-precision%29))
  (bind _returnvalue (Pawn|GetControlledPawn))
  (bind _targetplayer (Variables|Default|GetTargetPlayer))
  ;[0.15 0.15 0.15 0.5] No skippy attack
  (Networking|SwitchHasAuthority
    (:Authority
      (Utilities|IsValid (Variables|Default|GetTargetPlayer)
        (:Is%20Valid
          (bind _asbp_enemy_base (Utilities|Casting|CastToBP_EnemyBase (Pawn|GetControlledPawn)))
          (if (not (Math|Boolean|ORBoolean (Variables|/Game/DevLevels/Jays/Enemies/BP_EnemyBase.BP_EnemyBase_C|GetIsReacting _asbp_enemy_base) (Variables|/Game/DevLevels/Jays/Enemies/BP_EnemyBase.BP_EnemyBase_C|GetIsAttacking _asbp_enemy_base) (Variables|/Game/DevLevels/Jays/Enemies/BP_EnemyBase.BP_EnemyBase_C|GetIsDead _asbp_enemy_base)))
            (if (<= (Transformation|GetDistanceTo _returnvalue _targetplayer) (Variables|Default|GetAttackRange))
              ;[0.15 0.15 0.15 0.5] Target checks
              (Transformation|SetActorRotation _returnvalue (Math|Interpolation|RInterpTo (Transformation|GetActorRotation _returnvalue) (Math|Rotator|MakeRotator 0.0 0.0 (.Yaw (Math|Rotator|BreakRotator (Math|Rotator|FindLookatRotation (Transformation|GetActorLocation _returnvalue) (Transformation|GetActorLocation _targetplayer))))) DeltaSeconds 5.0)))))))))

(event EventBeginPlay
  ;[0.15 0.15 0.15 0.5] BeginPlay
  (Utilities|FlowControl|Delay 0.2)
  (CallFunction|TryPatrol))

(event EventPossess
  (params (PossessedPawn :type Pawn%20Object%20Reference))
  ;[0.15 0.15 0.15 0.5] Find nearest / chase nearest
  (Networking|SwitchHasAuthority
    (:Authority
      (CallFunction|FindNearestPlayer)
      (CallFunction|ChaseTarget)
      (Utilities|Time|SetTimerbyEvent (EventDispatchers|CreateEvent :!event Custom|CheckTarget) 0.5 true))))

(fn ConstructionScript)

(fn FindNearestPlayer
  (Variables|Default|SetTargetPlayer 0)
  (Variables|Default|SetClosestDistance 1e+09)
  (bind _outactors (Actor|GetAllActorsOfClass "/Game/Blueprints/PlayableCharacters/BP_BasePlayableCharacter.BP_BasePlayableCharacter_C"))
  (for _array_element _outactors
    (bind _asbp_base_playable_character (Utilities|Casting|CastToBP_BasePlayableCharacter _array_element))
    (if (Pawn|IsPlayerControlled _asbp_base_playable_character)
      (if (<= (Transformation|GetDistanceTo (Pawn|GetControlledPawn) _asbp_base_playable_character) (Variables|Default|GetDetectionRadius))
        (if (< (Transformation|GetDistanceTo (Pawn|GetControlledPawn) _asbp_base_playable_character) (Variables|Default|GetClosestDistance))
          (Variables|Default|SetClosestDistance (Transformation|GetDistanceTo (Pawn|GetControlledPawn) _asbp_base_playable_character))
          (Variables|Default|SetTargetPlayer _asbp_base_playable_character)
          (bind _asbp_enemy_base (Utilities|Casting|CastToBP_EnemyBase (Pawn|GetControlledPawn)))
          (Variables|/Game/DevLevels/Jays/Enemies/BP_EnemyBase.BP_EnemyBase_C|SetIsAlerted _asbp_enemy_base true))))))